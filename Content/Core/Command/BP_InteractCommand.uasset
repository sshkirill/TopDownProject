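; BP_InteractCommand is a command that makes an executor interact with a target actor.
; Execute calls the parent, then checks whether the valid target lies within InteractionRange.
; In range, it interacts through interface messages if the target allows it; otherwise it binds a move-finished event and sends the executor's BP_MovementComponent toward the target.
; The move-finished handler switches on the result but has no follow-up logic, so arrival triggers no interaction.
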(event Custom|OnInteractionMoveFinished
  (params (Result :type E_MovementResult%20Enum :default "NewEnumerator0"))
  (switch Utilities|FlowControl|Switch|SwitchonE_MovementResult Result))

(fn Execute
  (params (Executor :type Actor%20Object%20Reference))
  (bind _returnvalue (Actor|GetComponentbyClass Executor "/Game/Player/Components/BP_MovementComponent.BP_MovementComponent_C"))
  (bind _targetactor (Variables|Default|GetTargetActor))
  (bind _targetactor_2 (Variables|Default|GetTargetActor))
  (|CallParentFunction Executor)
  (if (Utilities|IsValid _targetactor)
    (if (== (Math|Float|Max(Float) 0.0 (- (Math|Vector|Distance(Vector) (Transformation|GetActorLocation _targetactor) (Transformation|GetActorLocation Executor)) (Variables|Default|GetInteractionRange))) 0.0)
      (bind _caninteract (Class|BPIInteractable|CanInteract(Message) _targetactor_2))
      (if _caninteract
        (Class|BPIInteractable|Interact(Message) (Variables|Default|GetTargetActor) Executor))
      (else
        (EventDispatchers|BindEventtoOnMoveFinished _returnvalue (EventDispatchers|CreateEvent :!event Custom|OnInteractionMoveFinished))
        (Default|MovetoActor _returnvalue _targetactor_2)))))