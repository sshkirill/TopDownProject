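; BP_MoveCommand is a command that moves its executor to a target location.
; Execute calls the parent, binds to the move-finished event on the executor's BP_MovementComponent, then starts MoveToLocation.
; An event handler prints the move result and maps success, failure or cancellation to the command's State.
; Cancel calls the parent and stops the component's movement.
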(event Custom|CustomEvent
  (params (Result :type E_MovementResult%20Enum :default "NewEnumerator0"))
  (Development|PrintString 0 (Utilities|String|EnumtoString Result))
  (switch Utilities|FlowControl|Switch|SwitchonE_MovementResult Result
    (:NewEnumerator0
      (Variables|Default|SetState "NewEnumerator2"))
    (:NewEnumerator1
      (Variables|Default|SetState "NewEnumerator4"))
    (:NewEnumerator2
      (Variables|Default|SetState "NewEnumerator3"))))

(fn Execute
  (params (Executor :type Actor%20Object%20Reference))
  (bind _returnvalue (Actor|GetComponentbyClass Executor "/Game/Player/Components/BP_MovementComponent.BP_MovementComponent_C"))
  (|CallParentFunction Executor)
  (EventDispatchers|BindEventtoOnMoveFinished _returnvalue (EventDispatchers|CreateEvent :!event Custom|CustomEvent))
  (Default|MovetoLocation _returnvalue (Variables|Default|GetTargetLocation)))

(fn Cancel
  (params (executor :type Actor%20Object%20Reference))
  (|CallParentFunction executor)
  (Default|StopMovement (Actor|GetComponentbyClass executor "/Game/Player/Components/BP_MovementComponent.BP_MovementComponent_C")))