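; BP_CommandExecutorComponent is an actor component that runs one command object at a time on its owning actor.
; ExecuteCommand cancels any current command, stores the new one and calls Execute on it with the owner.
; CancelCurrentCommand calls Cancel on a valid stored command with the owner, then clears the reference.
; The component delegates all behavior to the command objects, following the Command pattern, and has no active BeginPlay or Tick logic.
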(event EventBeginPlay)

(event EventTick
  (params (DeltaSeconds :type Float%20%28single-precision%29)))

(fn ExecuteCommand
  (params (command :type BP%20Gameplay%20Command%20Object%20Reference))
  (CallFunction|CancelCurrentCommand)
  (bind _output_get (Variables|Default|SetCurrentCommand command))
  (Default|Execute _output_get (Components|GetOwner)))

(fn CancelCurrentCommand
  (if (Utilities|IsValid (Variables|Default|GetCurrentCommand))
    (Default|Cancel (Variables|Default|GetCurrentCommand) (Components|GetOwner))
    (Variables|Default|SetCurrentCommand 0)))