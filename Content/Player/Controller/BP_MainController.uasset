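; Player controller for a click-driven RPG that spawns a separate camera actor, makes it the view target and smoothly follows the pawn each tick.
; BeginPlay also adds the player input mapping context and shows the cursor with Game and UI input.
; On primary click, the pawn's action resolver classifies the actor under the cursor as Move or Interact.
; The controller then builds the matching command object and passes it to the pawn's command executor.
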(event Input|EnhancedActionEvents|EnhancedInputActionIA_PrimaryAction
  (params (ActionValue :type Boolean) (ElapsedSeconds :type Float%20%28double-precision%29) (TriggeredSeconds :type Float%20%28double-precision%29) (InputAction :type Input%20Action%20Object%20Reference :default "/Game/Player/Input/IA_PrimaryAction.IA_PrimaryAction"))
  (bind _hitresult (Game|Player|GetHitResultUnderCursorbyChannel "TraceTypeQuery1" true))
  (bind (_bblockinghit _binitialoverlap _time _distance _location _impactpoint _normal _impactnormal _physmat _hitactor) (Collision|BreakHitResult _hitresult))
  (:Started
    (bind _action (Default|ResolveAction (Actor|GetComponentbyClass (Pawn|GetControlledPawn) "/Game/Core/Components/BP_ActionResolverComponent.BP_ActionResolverComponent_C") _hitactor))
    (switch Utilities|FlowControl|Switch|SwitchonE_PlayerAction _action
      (:NewEnumerator1
        (bind _returnvalue (Game|ConstructObjectfromClass "/Game/Core/Command/BP_MoveCommand.BP_MoveCommand_C"))
        (Variables|/Game/Core/Command/BP_MoveCommand.BP_MoveCommand_C|SetTargetLocation _returnvalue _impactpoint)
        (Default|ExecuteCommand (Actor|GetComponentbyClass (Pawn|GetControlledPawn) "/Game/Core/Components/BP_CommandExecutorComponent.BP_CommandExecutorComponent_C") _returnvalue))
      (:NewEnumerator2
        (bind _returnvalue_2 (Game|ConstructObjectfromClass "/Game/Core/Command/BP_InteractCommand.BP_InteractCommand_C"))
        (Variables|/Game/Core/Command/BP_InteractCommand.BP_InteractCommand_C|SetTargetActor _returnvalue_2 _hitactor)
        (Default|ExecuteCommand (Actor|GetComponentbyClass (Pawn|GetControlledPawn) "/Game/Core/Components/BP_CommandExecutorComponent.BP_CommandExecutorComponent_C") _returnvalue_2)))))

(event EventBeginPlay
  (bind _returnvalue (Game|SpawnActorfromClass "/Game/Player/Camera/BP_RPGCamera.BP_RPGCamera_C" (Math|Transform|MakeTransform (Transformation|GetActorLocation (Pawn|GetControlledPawn)) "0, 0, 0" "1.000000,1.000000,1.000000") "Undefined" "MultiplyWithRoot" 0 0))
  (bind _output_get (Variables|Default|SetRPGCamera _returnvalue))
  (Game|Player|SetViewTargetwithBlend (Game|GetPlayerController 0) _output_get 0.0 "VTBlend_Linear" 0.0 false)
  (Utilities|FlowControl|Sequence
    (:then_0
      (Input|AddMappingContext (PlayerController|LocalPlayerSubsystems|GetEnhancedInputLocalPlayerSubsystem self) "/Game/Player/Input/IMC_Player.IMC_Player" 0 "(bIgnoreAllPressedKeysUntilRelease=True,bForceImmediately=False,bNotifyUserSettings=False)"))
    (:then_1
      (Variables|Default|SetbShowMouseCursor true)
      (Input|SetInputModeGameandUI self 0 "DoNotLock" false false))))

(event EventTick
  (params (DeltaSeconds :type Float%20%28single-precision%29))
  (CallFunction|UpdateCameraPosition DeltaSeconds))

(fn ConstructionScript)

(fn UpdateCameraPosition
  (params (seconds :type Float%20%28double-precision%29))
  (bind _rpgcamera (Variables|Default|GetRPGCamera))
  (Transformation|SetActorLocation _rpgcamera (Math|Interpolation|VInterpTo (Transformation|GetActorLocation _rpgcamera) (Transformation|GetActorLocation (Pawn|GetControlledPawn)) seconds 5.0) false false))