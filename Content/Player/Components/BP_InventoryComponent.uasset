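; Player inventory component that stores items in a fixed number of slots, each holding an item ID and quantity.
; On BeginPlay it fills Slots with MaxSlots empty entries, marked by a "None" ID.
; AddItem reads the max stack size from BPItemSubSystem's item definition, then tops up matching stacks before filling empty slots.
; It returns the quantity left after the empty-slot pass, or the full quantity for an invalid definition.
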(event EventBeginPlay
  (CallFunction|InitializeInventory))

(event EventTick
  (params (DeltaSeconds :type Float%20%28single-precision%29)))

(fn AddItem
  (params (ItemID :type Name) (Quantity :type Integer))
  (Variables|Default|SetRemainingQuantity Quantity)
  (bind _itemdefinition (Default|GetItemDefinition (Subsystems|GetBPItemSubSystem) ItemID))
  (if (Utilities|IsValid _itemdefinition)
    (bind _output_get (LocalVariables|SetMaxStackSize (Variables|/Game/Core/Data/Items/Definitions/DA_ItemDefinition.DA_ItemDefinition_C|GetMaxStackSize _itemdefinition)))
    (for (_array_element _array_index) (Variables|Default|GetSlots)
      (if (and (== ItemID (.ItemID (Utilities|Struct|BreakST_InventorySlot _array_element))) (< (.Quantity (Utilities|Struct|BreakST_InventorySlot _array_element)) _output_get))
        (bind _output_get_2 (LocalVariables|Setspace (- (LocalVariables|GetMaxStackSize) (.Quantity (Utilities|Struct|BreakST_InventorySlot _array_element)))))
        (bind _output_get_3 (LocalVariables|SetAdded (+ (Math|Integer|Min(Integer) (Variables|Default|GetRemainingQuantity) _output_get_2) (.Quantity (Utilities|Struct|BreakST_InventorySlot _array_element)))))
        (bind _structout (Utilities|Struct|SetmembersinST_InventorySlot _array_element _output_get_3))
        (Utilities|Array|SetArrayElem (Variables|Default|GetSlots) _array_index _structout)
        (Variables|Default|SetRemainingQuantity (- (LocalVariables|GetAdded) (Variables|Default|GetRemainingQuantity)))))
    (if (> (Variables|Default|GetRemainingQuantity) 0)
      (for (_array_element_2 _array_index_2) (Variables|Default|GetSlots)
        (if (and (> (Variables|Default|GetRemainingQuantity) 0) (== (.ItemID (Utilities|Struct|BreakST_InventorySlot _array_element_2)) ""))
          (Utilities|Array|SetArrayElem (Variables|Default|GetSlots) _array_index_2 (Utilities|Struct|MakeST_InventorySlot ItemID (Math|Integer|Min(Integer) (Variables|Default|GetRemainingQuantity) (LocalVariables|GetMaxStackSize))))
          (Variables|Default|SetRemainingQuantity (- (Variables|Default|GetRemainingQuantity) (Math|Integer|Min(Integer) (Variables|Default|GetRemainingQuantity) (LocalVariables|GetMaxStackSize))))))
      (if (> (Variables|Default|GetRemainingQuantity) 0)
        (return (Variables|Default|GetRemainingQuantity))
        (else
          (return (Variables|Default|GetRemainingQuantity)))))
    (else
      (return Quantity))))

(fn InitializeInventory
  (Utilities|Array|Clear (Variables|Default|GetSlots))
  (for _index (range 0 (- (Variables|Default|GetMaxSlots) 1))
    (Utilities|Array|Add (Variables|Default|GetSlots) (Utilities|Struct|MakeST_InventorySlot "None"))))