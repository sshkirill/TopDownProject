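; Player movement component that sends its owning Pawn to a location or actor via SimpleMoveToLocation.
; MoveToLocation starts a looping timer that polls distance and velocity, firing OnMoveFinished with one result on arrival and another when the pawn stalls short.
; MoveToActor targets a point offset from the actor toward the pawn, without starting that check.
; StopMovement halts the controller and clears the timer.
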(event EventBeginPlay)

(event EventTick
  (params (DeltaSeconds :type Float%20%28single-precision%29)))

(fn MovetoLocation
  (params (TargetLocation :type Vector))
  (bind _output_get (Variables|Default|SetCurrentTargetLocation TargetLocation))
  (bind _aspawn (Utilities|Casting|CastToPawn (Components|GetOwner)))
  (AI|Navigation|SimpleMovetoLocation (Pawn|GetController _aspawn) _output_get)
  (bind _returnvalue (Utilities|Time|SetTimerbyFunctionName 0 "CheckMovement" 0.05 true))
  (Variables|Default|SetMovementCheckTimer _returnvalue))

(fn IsMoving
  (return (> (Math|Vector|VectorLength (Transformation|GetVelocity (Components|GetOwner))) 5.0)))

(fn CheckMovement
  (if (< (Math|Vector|Distance(Vector) (Variables|Default|GetCurrentTargetLocation) (Transformation|GetActorLocation (Components|GetOwner))) 1e+02)
    (Utilities|Time|ClearandInvalidateTimerbyHandle (Variables|Default|GetMovementCheckTimer))
    (Default|CallOnMoveFinished "NewEnumerator0")
    (else
      (bind _output (CallFunction|IsMoving))
      (if (not _output)
        (Utilities|Time|ClearandInvalidateTimerbyHandle (Variables|Default|GetMovementCheckTimer))
        (Default|CallOnMoveFinished "NewEnumerator1")))))

(fn StopMovement
  (bind _aspawn (Utilities|Casting|CastToPawn (Components|GetOwner)))
  (AI|Navigation|StopMovement (Pawn|GetController _aspawn))
  (Utilities|Time|ClearandInvalidateTimerbyHandle (Variables|Default|GetMovementCheckTimer)))

(fn MovetoActor
  (params (TargetActor :type Actor%20Object%20Reference))
  (bind _returnvalue (Transformation|GetActorLocation TargetActor))
  (bind _returnvalue_2 (Components|GetOwner))
  (bind _aspawn (Utilities|Casting|CastToPawn _returnvalue_2))
  (AI|Navigation|SimpleMovetoLocation (Pawn|GetController _aspawn) (+ _returnvalue (* (Math|Vector|Normalize (- (Transformation|GetActorLocation _returnvalue_2) _returnvalue)) 1.5e+02))))